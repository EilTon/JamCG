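; BP_Player is the player Blueprint that turns touch swipes into Up, Left or Right inputs for a timeline widget.
; On BeginPlay it takes the WidgetTimeline reference from BP_GameInstance.
; It records the first touch position on press and on release compares axis distances, treating a mostly upward swipe as Up and any other as Left or Right by X direction.
; The result goes to the widget's PlayerInput as an enum, with debug prints.
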(event `self.ReceiveBeginPlay`
  (bind _asbp_game_instance (cast `/Game/Blueprints/BP_GameInstance` (`GameplayStatics.GetGameInstance`)))
  (set `self.WidgetTimeline` (`/Game/Blueprints/BP_GameInstance.WidgetTimeline` _asbp_game_instance)))

(event `InputTouch`
  (params (Location :type "Vector Structure") (FingerIndex :type "ETouchIndex Enum"))
  (bind _widgettimeline (`self.WidgetTimeline`))
  (bind (_locationx _locationy) (`PlayerController.GetInputTouchState` (`GameplayStatics.GetPlayerController` 0) "Touch1"))
  (bind (_x _y) (`KismetMathLibrary.BreakVector2D` (`self.TouchEndXY`)))
  (bind (_x_2 _y_2) (`KismetMathLibrary.BreakVector2D` (`self.TouchBeginXY`)))
  (bind _returnvalue (`KismetMathLibrary.MakeVector2D` _locationx _locationy))
  (:`Pressed`
    (set `self.IsPressed` true)
    ;[1 1 1] Retrieve beginning of input
    (set `self.TouchBeginXY` _returnvalue))
  (:`Released`
    (if (`self.IsPressed`)
      (set `self.IsPressed` false)
      (bind _output_get (set `self.TouchEndXY` _returnvalue))
      (`KismetSystemLibrary.PrintString` (`KismetStringLibrary.Conv_Vector2dToString` _output_get) false false)
      (if (and (> _y_2 _y) (> (`KismetMathLibrary.Abs` (- _y_2 _y)) (`KismetMathLibrary.Abs` (- _x_2 _x))))
        (`KismetSystemLibrary.PrintString` "Up")
        (`/Game/Blueprints/WBP_Timeline.PlayerInput` _widgettimeline "NewEnumerator0")
        (elif (> _x_2 _x)
          (`KismetSystemLibrary.PrintString` "Left")
          (`/Game/Blueprints/WBP_Timeline.PlayerInput` _widgettimeline "NewEnumerator1")
          (else
            (`KismetSystemLibrary.PrintString` "Right")
            (`/Game/Blueprints/WBP_Timeline.PlayerInput` _widgettimeline "NewEnumerator2")))))))

(fn `UserConstructionScript`)