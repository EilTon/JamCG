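; BP_Opponent is an enemy caster that fires a timed series of random Fire, Water or Air spells on BeginPlay.
; A custom LoopWithDelay macro paces the attempts, each gated by a randomly weighted chance to cast.
; CastSpell spawns BP_Spell at the element's spot, and one shared MoveForward timeline lerps it along world X.
; Successful casts also animate an icon in WBP_SpawnSpellIcon and queue the element in WBP_Timeline.
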(event `Cast Spell`
  (params (Spot :type "SceneComponent Object Reference"))
  (bind _returnvalue (`SceneComponent.K2_GetComponentLocation` Spot))
  ;[1 1 1] Cast Spell
  (bind _returnvalue_2 (`|SpawnActorFromClass` "/Game/Blueprints/BP_Spell.BP_Spell_C" (`SceneComponent.K2_GetComponentToWorld` Spot) "Undefined" "OverrideRootScale" null null))
  (bind (_direction _lerp) (`Timeline|MoveForward` :!via `PlayFromStart`)
    (:`Update`
      (`self.K2_SetActorRelativeLocation` _returnvalue_2 (`KismetMathLibrary.VLerp` _returnvalue (`KismetMathLibrary.MakeVector` (+ (.x _returnvalue) 1000.0) (.y _returnvalue) (.z _returnvalue)) _lerp) false false))))

(event `self.ReceiveBeginPlay`
  ;[1 1 1] Generations Seplls
  (bind _returnvalue (`|CreateWidget` "/Game/Blueprints/WBP_Timeline.WBP_Timeline_C"))
  (bind _output_get (set `self.WidgetTimeline` _returnvalue))
  (`UserWidget.AddToViewport` _output_get 0)
  (bind _returnvalue_2 (`|CreateWidget` "/Game/Blueprints/WBP_SpawnSpellIcon.WBP_SpawnSpellIcon_C"))
  (bind _output_get_2 (set `self.WidgetSpellIcon` _returnvalue_2))
  (`UserWidget.AddToViewport` _output_get_2 0)
  (`self.LoopWithDelay` 0 (- (`self.HowManySpellToCast`) 1) 0.6
    (:`Loop Body`
      (switch `int` (`KismetMathLibrary.RandomInteger` 3)
        (:`0`
          (set `self.SpellToCast` "NewEnumerator0"))
        (:`1`
          (set `self.SpellToCast` "NewEnumerator1"))
        (:`2`
          (set `self.SpellToCast` "NewEnumerator2")))
      (if (`KismetMathLibrary.RandomBoolWithWeight` (`KismetMathLibrary.RandomFloatInRange` (`self.WeightBoolMin`) (`self.WeightBoolMax`)))
        (switch `/Game/Blueprints/ESpell` (`self.SpellToCast`)
          (:`NewEnumerator0`
            (`self.Cast Spell` (`self.FireSpot`))
            (`/Game/Blueprints/WBP_SpawnSpellIcon.Move Image` (`self.WidgetSpellIcon`) (`|GetArrayItem` (`self.ImagesSpells`))))
          (:`NewEnumerator1`
            (`self.Cast Spell` (`self.WaterSpot`))
            (`/Game/Blueprints/WBP_SpawnSpellIcon.Move Image` (`self.WidgetSpellIcon`) (`|GetArrayItem` (`self.ImagesSpells`) 1)))
          (:`NewEnumerator2`
            (`self.Cast Spell` (`self.AirSpot`))
            (`/Game/Blueprints/WBP_SpawnSpellIcon.Move Image` (`self.WidgetSpellIcon`) (`|GetArrayItem` (`self.ImagesSpells`) 2))))
        (`/Game/Blueprints/WBP_Timeline.AddQueue` (`self.WidgetTimeline`) (`self.SpellToCast`))
        (else
          (`KismetSystemLibrary.PrintString` "No Spell"))))))

(fn `UserConstructionScript`)